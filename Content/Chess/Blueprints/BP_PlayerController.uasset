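; Player controller for a chess game that relays input to the game mode and drives the main HUD.
; Move-piece and camera-rotate inputs forward straight to BP_GameMode, which it caches during Initialize along with enabling input and the mouse cursor.
; It creates the UI_Main widget and UpdateUI pulls both players' info, the active color, move data and checkmate or stalemate status from the game mode into it.
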(event `InputAction|MoveChessPiece`
  (params (Key :type "Key Structure"))
  (:`Pressed`
    (`/Game/Chess/Blueprints/BP_GameMode.ProcessMove` (`self.GameModeRef`))))

(event `InputAxis|RotatePlayerCamera`
  (params (AxisValue :type "Float (single-precision)"))
  (`/Game/Chess/Blueprints/BP_GameMode.RotateCamera` (`self.GameModeRef`) AxisValue))

(fn `Initialize`
  (`|ExecutionSequence`
    (:`then_0`
      (`self.EnableInput` self)
      (set `self.bShowMouseCursor` true))
    (:`then_1`
      (`self.SetGameModeRef`)
      (`self.SetMainUI`))))

(fn `SetGameModeRef`
  (`/Engine/EditorBlueprintResources/StandardMacros.IsValid` (`self.GameModeRef`)
    (:`Is Not Valid`
      (bind _asbp_game_mode (cast `/Game/Chess/Blueprints/BP_GameMode` (`GameplayStatics.GetGameMode`)))
      (set `self.GameModeRef` _asbp_game_mode))))

(fn `SetMainUI`
  (bind _returnvalue (`|CreateWidget` "/Game/Chess/UI/UI_Main.UI_Main_C" self))
  (bind _output_get (set `self.MainUIRef` _returnvalue))
  (`UserWidget.AddToViewport` _output_get 0)
  (`/Game/Chess/UI/UI_Main.OpenUI` (`self.MainUIRef`))
  (`self.UpdateUI`))

(fn `SetMessage`
  (params (NewMessage :type String))
  (set `self.Message` NewMessage))

(fn `SetPlayerInfoInUI`
  (params (PlayerIndex :type Integer))
  (bind (_name _color _index _ischeckflag _haslegalmovesflag _movecount _captures) (break `/Game/Chess/Blueprints/ST_Player` (`/Game/Chess/Blueprints/BP_GameMode.GetPlayerByIndex` (`self.GameModeRef`) PlayerIndex)))
  (`/Game/Chess/UI/UI_Main.SetPlayerName` (`self.MainUIRef`) _color _name)
  (`/Game/Chess/UI/UI_Main.SetCheckStatus` (`self.MainUIRef`) _color _ischeckflag)
  (`/Game/Chess/UI/UI_Main.SetCaptureCounts` (`self.MainUIRef`) _color _captures))

(fn `UpdateUI`
  (bind _gamemoderef (`self.GameModeRef`))
  (bind (_ischeckmate _isstalemate) (`/Game/Chess/Blueprints/BP_GameMode.GetGameStatus` (`self.GameModeRef`)))
  (bind (_color _latestmovenotation) (`/Game/Chess/Blueprints/BP_GameMode.GetLatestMove` _gamemoderef))
  (`/Game/Chess/UI/UI_Main.SetActivePlayer` (`self.MainUIRef`) (`/Game/Chess/Blueprints/BP_GameMode.GetActivePlayerColor` (`self.GameModeRef`)))
  (`|ExecutionSequence`
    (:`then_0`
      (`self.SetPlayerInfoInUI` 0)
      (`self.SetPlayerInfoInUI` 1))
    (:`then_1`
      (`/Game/Chess/UI/UI_Main.SetMoveCount` (`self.MainUIRef`) (`/Game/Chess/Blueprints/BP_GameMode.GetMoveCount` _gamemoderef))
      (`/Game/Chess/UI/UI_Main.SetLatestMove` (`self.MainUIRef`) _color _latestmovenotation)
      (`/Game/Chess/UI/UI_Main.SetMessage1` (`self.MainUIRef`) (`self.Message`))
      (if _ischeckmate
        (`/Game/Chess/UI/UI_Main.SetMessage2` (`self.MainUIRef`) "Check Mate! Game Over!")
        (elif _isstalemate
          (`/Game/Chess/UI/UI_Main.SetMessage2` (`self.MainUIRef`) "Stale Mate! Game Over!")
          (else
            (`/Game/Chess/UI/UI_Main.SetMessage2` (`self.MainUIRef`) "")))))))

(fn `UserConstructionScript`)