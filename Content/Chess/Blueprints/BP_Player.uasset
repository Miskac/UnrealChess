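; Chess player Blueprint that holds both players' state and controls the board camera.
; Each player is an ST_Player struct, looked up by index or color, with setters rebuilding the whole struct to change name, color, check and legal-move flags, or move and capture counts.
; SetPlayerCamera eases the Azimuth pivot and glides the camera to the White or Black anchor transform, while RotateCamera yaws the pivot from axis input.
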(event `SetPlayerCamera`
  (params (Color :type "/Game/Chess/Blueprints/EN_Color Enum" :default "NewEnumerator0"))
  (bind (_returnvalue_location _returnvalue_rotation) (`KismetMathLibrary.BreakTransform` (`SceneComponent.GetRelativeTransform` (`self.Black`))))
  (bind (_returnvalue_location_2 _returnvalue_rotation_2) (`KismetMathLibrary.BreakTransform` (`SceneComponent.GetRelativeTransform` (`self.White`))))
  (`KismetSystemLibrary.MoveComponentTo` (`self.Azimuth`) (0.0 0.0 0.0) (struct) true true 1.0 true)
  (switch `/Game/Chess/Blueprints/EN_Color` Color
    (:`NewEnumerator0`
      (`KismetSystemLibrary.MoveComponentTo` (`self.Camera`) _returnvalue_location_2 _returnvalue_rotation_2 true true 3.0 true))
    (:`NewEnumerator1`
      (`KismetSystemLibrary.MoveComponentTo` (`self.Camera`) _returnvalue_location _returnvalue_rotation true true 3.0 true))))

(fn `GetPlayerByColor`
  (params (Color :type "/Game/Chess/Blueprints/EN_Color Enum" :default "NewEnumerator0"))
  (returns (Player :type "/Game/Chess/Blueprints/ST_Player Structure"))
  (bind (_player0ref_name _player0ref_color) (break `/Game/Chess/Blueprints/ST_Player` (`self.Player0Ref`)))
  (if (`|EnumEquality` Color _player0ref_color)
    (return (`self.Player0Ref`))
    (else
      (return (`self.Player1Ref`)))))

(fn `GetPlayerByIndex`
  (params (Index :type Integer))
  (returns (Player :type "/Game/Chess/Blueprints/ST_Player Structure"))
  (bind (_player0ref_name _player0ref_color _player0ref_index) (break `/Game/Chess/Blueprints/ST_Player` (`self.Player0Ref`)))
  (if (== Index _player0ref_index)
    (return (`self.Player0Ref`))
    (else
      (return (`self.Player1Ref`)))))

(fn `IncrmentPlayerCaptures`
  (params (PlayerIndex :type Integer))
  (bind (_name _color _index _ischeckflag _haslegalmovesflag _movecount _captures) (break `/Game/Chess/Blueprints/ST_Player` (`self.Player1Ref`)))
  (bind (_name_2 _color_2 _index_2 _ischeckflag_2 _haslegalmovesflag_2 _movecount_2 _captures_2) (break `/Game/Chess/Blueprints/ST_Player` (`self.Player0Ref`)))
  (switch `int` PlayerIndex
    (:`0`
      (set `self.Player0Ref` (make `/Game/Chess/Blueprints/ST_Player` _name_2 _color_2 _index_2 _ischeckflag_2 _haslegalmovesflag_2 _movecount_2 (+ _captures_2 1))))
    (:`1`
      (set `self.Player1Ref` (make `/Game/Chess/Blueprints/ST_Player` _name _color _index _ischeckflag _haslegalmovesflag _movecount (+ _captures 1))))))

(fn `IncrmentPlayerMoves`
  (params (PlayerIndex :type Integer))
  (bind (_name _color _index _ischeckflag _haslegalmovesflag _movecount _captures) (break `/Game/Chess/Blueprints/ST_Player` (`self.Player1Ref`)))
  (bind (_name_2 _color_2 _index_2 _ischeckflag_2 _haslegalmovesflag_2 _movecount_2 _captures_2) (break `/Game/Chess/Blueprints/ST_Player` (`self.Player0Ref`)))
  (switch `int` PlayerIndex
    (:`0`
      (set `self.Player0Ref` (make `/Game/Chess/Blueprints/ST_Player` _name_2 _color_2 _index_2 _ischeckflag_2 _haslegalmovesflag_2 (+ _movecount_2 1) _captures_2)))
    (:`1`
      (set `self.Player1Ref` (make `/Game/Chess/Blueprints/ST_Player` _name _color _index _ischeckflag _haslegalmovesflag (+ _movecount 1) _captures)))))

(fn `Initialize`)

(fn `RotateCamera`
  (params (Axis :type "Float (double-precision)"))
  (bind (_relativerotation_roll _relativerotation_pitch _relativerotation_yaw) (`KismetMathLibrary.BreakRotator` (`SceneComponent.RelativeRotation` (`self.Azimuth`))))
  (if (!= Axis 0.0)
    (`SceneComponent.K2_SetRelativeRotation` (`self.Azimuth`) (`KismetMathLibrary.MakeRotator` 0.0 0.0 (+ Axis _relativerotation_yaw)) false false)))

(fn `SetHasLegalMovesFlag`
  (params (PlayerIndex :type Integer) (HasLegalMovesFlag :type Boolean))
  (bind (_name _color _index _ischeckflag _haslegalmovesflag _movecount _captures) (break `/Game/Chess/Blueprints/ST_Player` (`self.Player1Ref`)))
  (bind (_name_2 _color_2 _index_2 _ischeckflag_2 _haslegalmovesflag_2 _movecount_2 _captures_2) (break `/Game/Chess/Blueprints/ST_Player` (`self.Player0Ref`)))
  (switch `int` PlayerIndex
    (:`0`
      (set `self.Player0Ref` (make `/Game/Chess/Blueprints/ST_Player` _name_2 _color_2 _index_2 _ischeckflag_2 HasLegalMovesFlag _movecount_2 _captures_2)))
    (:`1`
      (set `self.Player1Ref` (make `/Game/Chess/Blueprints/ST_Player` _name _color _index _ischeckflag HasLegalMovesFlag _movecount _captures)))))

(fn `SetKinginCheckFlag`
  (params (PlayerIndex :type Integer) (IsCheckFlag :type Boolean))
  (bind (_name _color _index _ischeckflag _haslegalmovesflag _movecount _captures) (break `/Game/Chess/Blueprints/ST_Player` (`self.Player1Ref`)))
  (bind (_name_2 _color_2 _index_2 _ischeckflag_2 _haslegalmovesflag_2 _movecount_2 _captures_2) (break `/Game/Chess/Blueprints/ST_Player` (`self.Player0Ref`)))
  (switch `int` PlayerIndex
    (:`0`
      (set `self.Player0Ref` (make `/Game/Chess/Blueprints/ST_Player` _name_2 _color_2 _index_2 IsCheckFlag _haslegalmovesflag_2 _movecount_2 _captures_2)))
    (:`1`
      (set `self.Player1Ref` (make `/Game/Chess/Blueprints/ST_Player` _name _color _index IsCheckFlag _haslegalmovesflag _movecount _captures)))))

(fn `SetPlayerColor`
  (params (PlayerIndex :type Integer) (Color :type "/Game/Chess/Blueprints/EN_Color Enum" :default "NewEnumerator0"))
  (bind (_name _color _index _ischeckflag _haslegalmovesflag _movecount _captures) (break `/Game/Chess/Blueprints/ST_Player` (`self.Player1Ref`)))
  (bind (_name_2 _color_2 _index_2 _ischeckflag_2 _haslegalmovesflag_2 _movecount_2 _captures_2) (break `/Game/Chess/Blueprints/ST_Player` (`self.Player0Ref`)))
  (switch `int` PlayerIndex
    (:`0`
      (set `self.Player0Ref` (make `/Game/Chess/Blueprints/ST_Player` _name_2 Color _index_2 _ischeckflag_2 _haslegalmovesflag_2 _movecount_2 _captures_2)))
    (:`1`
      (set `self.Player1Ref` (make `/Game/Chess/Blueprints/ST_Player` _name Color _index _ischeckflag _haslegalmovesflag _movecount _captures)))))

(fn `SetPlayerName`
  (params (PlayerIndex :type Integer) (Name :type String))
  (bind (_name _color _index _ischeckflag _haslegalmovesflag _movecount _captures) (break `/Game/Chess/Blueprints/ST_Player` (`self.Player1Ref`)))
  (bind (_name_2 _color_2 _index_2 _ischeckflag_2 _haslegalmovesflag_2 _movecount_2 _captures_2) (break `/Game/Chess/Blueprints/ST_Player` (`self.Player0Ref`)))
  (switch `int` PlayerIndex
    (:`0`
      (set `self.Player0Ref` (make `/Game/Chess/Blueprints/ST_Player` Name _color_2 _index_2 _ischeckflag_2 _haslegalmovesflag_2 _movecount_2 _captures_2)))
    (:`1`
      (set `self.Player1Ref` (make `/Game/Chess/Blueprints/ST_Player` Name _color _index _ischeckflag _haslegalmovesflag _movecount _captures)))))

(fn `UserConstructionScript`)